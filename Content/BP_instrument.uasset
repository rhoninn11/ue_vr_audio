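; Playable instrument actor that lines a spline with miniature musical obelisks laid out like piano keys and relays their hits to a haptic hub.
; On construction, 12-key octave lookup maps set each key's distance and raised offset, stopping at the spline's length, with semitone tones numbered by spawn order.
; At BeginPlay it finds BP_haptic_hub, binds each obelisk's note-hit event a tick later, and forwards pitch, ignoring velocity.
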(event `on_construct`
  (`self.spawn_note_bricks_along_spline`))

(event `self.ReceiveBeginPlay`
  (`|ExecutionSequence`
    (:`then_0`
      (bind _returnvalue (`GameplayStatics.GetActorOfClass` "/sound_experiment/haptics/BP_haptic_hub.BP_haptic_hub_C"))
      (set `self.haptic_hub_connection` _returnvalue))
    (:`then_1`
      (`KismetSystemLibrary.DelayUntilNextTick`)
      (for _array_element (`self.dynamicaly_spawned`)
        (add `/sound_experiment/BP_obelisk_muzyczny.note_hit` _array_element (delegate `on_hit_note`))))))

(event `on_hit_note`
  (params (pitch :type "Float (double-precision)") (velocity :type "Float (double-precision)"))
  (`/Engine/EditorBlueprintResources/StandardMacros.IsValid` (`self.haptic_hub_connection`)
    (:`Is Valid`
      (`/sound_experiment/haptics/BP_haptic_hub.play_pitch` (`self.haptic_hub_connection`) pitch))))

(fn `keyboard_spacing`
  (params (key_idx :type Integer))
  (returns (distance_units :type "Float (double-precision)") (bump_units :type "Float (double-precision)"))
  (locals (along_map :type "Array of Float (double-precision)") (bumped_map :type "Array of Float (double-precision)"))
  (bind _returnvalue (mod key_idx 12))
  (return (+ (`|GetArrayItem` (`local.along_map`) _returnvalue) (* 7.0 (`KismetMathLibrary.FFloor` (/ key_idx 12)))) (`|GetArrayItem` (`local.bumped_map`) _returnvalue)))

(fn `spawn_note_bricks_along_spline`
  (bind _spline (`self.Spline`))
  (bind _tile_spaceing (`self.tile_spaceing`))
  (`KismetArrayLibrary.Array_Clear` (`self.dynamicaly_spawned`))
  (for _index (range (* 12 (`self.octave_num`)))
    (bind (_distance_units _bump_units) (`self.keyboard_spacing` _index))
    (bind _returnvalue (* _distance_units _tile_spaceing))
    (if (< _returnvalue (`SplineComponent.GetSplineLength` (`self.Spline`)))
      (bind _returnvalue_2 (`SplineComponent.GetRotationAtDistanceAlongSpline` _spline _returnvalue "Local"))
      ;[1 1 1] creation and config of next tile
      (bind _returnvalue_3 (`AddComponent|NODE_AddChildActorComponent-0` :`RelativeTransform` (`KismetMathLibrary.MakeTransform` (+ (`SplineComponent.GetLocationAtDistanceAlongSpline` _spline _returnvalue "Local") (* (+ (* (`KismetMathLibrary.GetUpVector` _returnvalue_2) (`KismetMathLibrary.Conv_DoubleToVector` 2.0)) (* (`KismetMathLibrary.GetRightVector` _returnvalue_2) (`KismetMathLibrary.Conv_DoubleToVector` -1.0))) (* _bump_units _tile_spaceing))) (`KismetMathLibrary.ComposeRotators` (`KismetMathLibrary.MakeRotator` -75.0) _returnvalue_2) (`KismetMathLibrary.Conv_DoubleToVector` 0.1))))
      (`ChildActorComponent.SetChildActorClass` _returnvalue_3 "/sound_experiment/BP_obelisk_muzyczny.BP_obelisk_muzyczny_C")
      (bind _asbp_obelisk_muzyczny (cast `/sound_experiment/BP_obelisk_muzyczny` (`ChildActorComponent.ChildActor` _returnvalue_3)))
      (bind _returnvalue_4 (`KismetArrayLibrary.Array_Add` (`self.dynamicaly_spawned`) _asbp_obelisk_muzyczny))
      (set `/sound_experiment/BP_obelisk_muzyczny.tone` (`KismetMathLibrary.Conv_IntToDouble` (+ _returnvalue_4 -24)) _asbp_obelisk_muzyczny))))

(fn `UserConstructionScript`
  (`self.spawn_note_bricks_along_spline`))