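; Musical brick actor that wobbles when it receives a note and passes that note on with its own tone.
; At construction and BeginPlay it registers as receiver with its Muzyczny child actor and sends it HitTone.
; ReciveNote logs the velocity, starts the wobble and forwards tone and velocity to the assigned BroadcastBro.
; Tick scales the mesh along the WobblyShape curve, weighted by velocity, for one second.
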(event `self.ReceiveBeginPlay`
  (bind _childactor (`ChildActorComponent.ChildActor` (`self.muzyczny`)))
  (`|ExecutionSequence`
    (:`then_0`
      (set `self.reference_brick_scale` (.scale (`SceneComponent.GetRelativeTransform` (`self.brick_like_mesh`)))))
    (:`then_1`
      (message `/mea_vr_audio/BPI_melodic_hit._add_reciver` _childactor self :!label _label)
      (message `/mea_vr_audio/BPI_melodic_hit._set_tone` _childactor (`self.hit_tone`)))))

(event `on_construct`
  (goto _label))

(event `/mea_vr_audio/haptics/BPI_note_recive._recive_note`
  (params (pitch :type "Float (double-precision)") (velocity :type "Float (double-precision)"))
  (set `self.hit_velocity` velocity)
  (message `/mea_vr_audio/log/BPI_logs.add_log` (`self.log_to`) (`KismetStringLibrary.Concat_StrStr` "+++ my hit velocity is: " (`KismetStringLibrary.Conv_DoubleToString` velocity)))
  (`|ExecutionSequence`
    (:`then_0`
      ;[1 1 1] wobble_init
      (`|ExecutionSequence`
        (:`then_0`
          (set `self.wobblying` true)
          (set `self.wobbly_time` 0.0))
        (:`then_1`
          (set `self.wobbly_strength` (`self.hit_velocity`)))))
    (:`then_1`
      (message `/mea_vr_audio/haptics/BPI_note_recive._recive_note` (`self.broadcast_bro`) (`self.hit_tone`) (`self.hit_velocity`)))))

(event `self.ReceiveTick`
  (params (DeltaSeconds :type "Float (single-precision)"))
  ;[0.3516 0.2319 1] wobbling_process
  (if (`self.wobblying`)
    (`|ExecutionSequence`
      (:`then_0`
        ;;[0.01485 0.3021 0] time passing
        (set `self.wobbly_time` (+ DeltaSeconds (`self.wobbly_time`))))
      (:`then_1`
        ;;[1 1 1] play wobbly animation
        (`SceneComponent.SetRelativeScale3D` (`self.brick_like_mesh`) (* (+ (* (`CurveFloat.GetFloatValue` (`self.wobbly_shape`) (`self.wobbly_time`)) (`self.wobbly_strength`)) 1.0) (`self.reference_brick_scale`))))
      (:`then_2`
        ;;[1 1 1] pause wobblig process
        (if (> (`self.wobbly_time`) 1.0)
          (set `self.wobblying` false)
          (set `self.wobbly_time` 0.0))))))

(event `/mea_vr_audio/haptics/BPI_note_recive._add_broadcast_bro`
  (params (bro :type "Actor Object Reference"))
  (set `self.broadcast_bro` bro))

(fn `UserConstructionScript`
  (`self.on_construct`))