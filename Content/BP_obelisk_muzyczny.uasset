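; Musical obelisk actor that plays a set pitch and wobbles when struck.
; Passes its Tone to a BP_sound_collision child actor and binds to that actor's trigger, both on construction and at BeginPlay.
; A trigger calls NoteHit with pitch and velocity, then Tick pulses the obelisk's scale for about one second using the WobblyShape curve scaled by hit velocity.
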(event `on_construct`
  ;[1 1 1] Comment
  (bind _asbp_sound_collision (cast `/sound_experiment/BP_sound_collision` (`ChildActorComponent.ChildActor` (`self.muzyczny`)) :!label _label))
  (add `/sound_experiment/BP_sound_collision.other_reactons` _asbp_sound_collision (delegate `actor_triggered`))
  ;[1 1 1] this obelisk pitch
  (`/sound_experiment/BP_sound_collision.set_tone` _asbp_sound_collision (`self.tone`)))

(event `self.ReceiveBeginPlay`
  (goto _label))

(event `actor_triggered`
  (params (vel :type "Float (double-precision)"))
  ;[1 1 1] wobble_init
  (`|ExecutionSequence`
    (:`then_0`
      (set `self.wobblying` true)
      (set `self.wobbly_time` 0.0))
    (:`then_1`
      (set `self.wobbly_strength` vel))
    (:`then_2`
      (`self.note_hit` (`self.tone`) vel))))

(event `self.ReceiveTick`
  (params (DeltaSeconds :type "Float (single-precision)"))
  ;[0.3516 0.2319 1] wobbling_process
  (if (`self.wobblying`)
    (`|ExecutionSequence`
      (:`then_0`
        ;;[0.01485 0.3021 0] time passing
        (set `self.wobbly_time` (+ DeltaSeconds (`self.wobbly_time`))))
      (:`then_1`
        ;;[1 1 1] play wobbly animation
        (`SceneComponent.SetRelativeScale3D` (`self.obelisk`) (`KismetMathLibrary.Conv_DoubleToVector` (+ (* (`CurveFloat.GetFloatValue` (`self.wobbly_shape`) (`self.wobbly_time`)) (`self.wobbly_strength`)) 1.0))))
      (:`then_2`
        ;;[1 1 1] pause wobblig process
        (if (> (`self.wobbly_time`) 1.0)
          (set `self.wobblying` false)
          (set `self.wobbly_time` 0.0))))))

(fn `UserConstructionScript`
  (`self.on_construct`))