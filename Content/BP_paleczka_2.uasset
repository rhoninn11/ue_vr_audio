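; BP_paleczka_2 is a grabbable stick actor ("pałeczka") that gives haptic feedback through its sound-collision component.
; On BeginPlay it casts its child actor to BP_sound_collision and binds an event to that actor's OtherReactons hook.
; That event plays a haptic effect on the hand reported by GrabComponent, ignoring the passed velocity.
; Grab and drop events toggle GrabFlag, and the construction script constructs a BP_avg_vel_calculator.
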(event `self.ReceiveBeginPlay`
  (`|ExecutionSequence`
    (:`then_0`
      (bind _asbp_sound_collision (cast `/sound_experiment/BP_sound_collision` (`ChildActorComponent.ChildActor` (`self.BP_sound_collision`))))
      (set `self.sound_colison` _asbp_sound_collision))
    (:`then_1`
      (add `/sound_experiment/BP_sound_collision.other_reactons` (`self.sound_colison`) (delegate `CustomEvent`)))))

(event `self.ReceiveTick`
  (params (DeltaSeconds :type "Float (single-precision)")))

(event `CustomEvent`
  (params (vel :type "Float (double-precision)"))
  ;[0.03434 0.03434 0.03434] Play Haptic Effect
  (`PlayerController.PlayHapticEffect` (`GameplayStatics.GetPlayerController` 0) "/sound_experiment/haptics/buffor_haptic_test.buffor_haptic_test" (`/Game/VRTemplate/Blueprints/GrabComponent.GetHeldByHand` (`self.GrabComponent`)) 1.0 false))

(event `self.GrabComponent.OnGrabbed`
  ;[1 1 1] grab_indicator
  (set `self.grab_flag` true))

(event `self.GrabComponent.OnDropped`
  ;[1 1 1] grab_indicator
  (set `self.grab_flag` false))

(fn `UserConstructionScript`
  (`|GenericCreateObject` "/vr_sound_interactions/muzyczne_demo/BP_avg_vel_calculator.BP_avg_vel_calculator_C"))