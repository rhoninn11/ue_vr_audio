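; Sound collision actor whose capsule reacts when an overlapping component tagged "trigger_sound" enters it.
; The overlapping actor's speed is scaled and clamped into a Velocity value that serves as volume.
; If Audible, it passes that volume and a settable tone to an audio source as parameters and plays it; if Active, it forwards Velocity to a reaction chain.
; The construction script sets capsule half-height from a shape alpha.
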(event `self.ReceiveBeginPlay`)

(event `self.Capsule.OnComponentBeginOverlap`
  (params (OverlappedComponent :type "PrimitiveComponent Object Reference") (OtherActor :type "Actor Object Reference") (OtherComp :type "PrimitiveComponent Object Reference") (OtherBodyIndex :type Integer) (bFromSweep :type Boolean) (SweepResult :type "HitResult Structure (by ref)"))
  (bind _simple_effect_play (`self.simple_effect_play`))
  (if (`ActorComponent.ComponentHasTag` OtherComp "trigger_sound")
    (`|ExecutionSequence`
      (:`then_0`
        ;[1 1 1] velocity_probe
        (set `self.velocity` (`KismetMathLibrary.FClamp` (/ (`KismetMathLibrary.VSize` (`self.GetVelocity` OtherActor)) 100.0) 0.1 2.0)))
      (:`then_1`
        ;[1 1 1] audio reaction
        (if (`self.audible`)
          (`|ExecutionSequence`
            (:`then_0`
              (`self.apply_audio_parameters` _simple_effect_play))
            (:`then_1`
              (`AudioComponent.Play` _simple_effect_play 0.0)))))
      (:`then_2`
        ;[1 1 1] activate reaction chain
        (if (`self.active`)
          (`self.other_reactons` (`self.velocity`)))))))

(fn `apply_audio_parameters`
  (params (sound_source :type "AudioComponent Object Reference"))
  (`AudioComponent.SetFloatParameter` sound_source "base_tone" (`self.tone`))
  (`AudioComponent.SetFloatParameter` sound_source "volume" (`self.velocity`)))

(fn `set_tone`
  (params (tone :type "Float (double-precision)"))
  (set `self.tone` tone)
  (`self.apply_audio_parameters` (`self.simple_effect_play`)))

(fn `UserConstructionScript`
  (`CapsuleComponent.SetCapsuleHalfHeight` (`self.Capsule`) (`KismetMathLibrary.Lerp` 45.0 120.0 (`self.capsule_shape`)) false))