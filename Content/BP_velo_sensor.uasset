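; Velocity sensor that estimates the direction and speed of its own movement from world-position changes.
; Each Tick, PosUpdate shifts a three-sample history of positions and frame times.
; Direction is the normalized sum of the last two displacements, and speed averages both intervals in meters per second, with an epsilon guarding against division by zero.
; GetVelocity exposes the stored direction and speed.
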(event `self.ReceiveTick`
  (params (DeltaSeconds :type "Float (single-precision)"))
  ;[1 1 1] update block
  (bind (_velo_dir_out _velo_value_out) (`self.pos_update` (`self.K2_GetComponentLocation` self) DeltaSeconds))
  (set `self.velocity_dir` _velo_dir_out)
  (set `self.velocity_value` _velo_value_out))

(fn `get_velocity`
  (returns (velocity_value :type "Float (double-precision)") (velocity_dir :type "Vector Structure"))
  (return (`self.velocity_value`) (`self.velocity_dir`)))

(fn `pos_update`
  (params (pos :type "Vector Structure") (delta :type "Float (double-precision)"))
  (returns (velo_dir_out :type "Vector Structure") (velo_value_out :type "Float (double-precision)"))
  (locals (velo_vector :type "Vector Structure") (velo_value :type "Float (double-precision)"))
  (bind _pos_last (`self.pos_last`))
  (bind _returnvalue (- _pos_last (`self.pos_last_last`)))
  (bind _returnvalue_2 (- (`self.pos_now`) _pos_last))
  (`|ExecutionSequence`
    (:`then_0`
      ;[1 1 1] update pos
      (set `self.pos_last_last` (`self.pos_last`))
      (set `self.pos_last` (`self.pos_now`))
      (set `self.pos_now` pos))
    (:`then_1`
      ;[1 1 1] update time
      (set `self.delta_last_last` (`self.delta_last`))
      (set `self.delta_last` (`self.delta_now`))
      (set `self.delta_now` delta))
    (:`then_2`
      ;[1 1 1] calc
      (set `local.velo_vector` (`KismetMathLibrary.Normal` (+ _returnvalue_2 _returnvalue)))
      (set `local.velo_value` (/ (/ (+ (/ (`KismetMathLibrary.VSize` _returnvalue_2) (+ (`self.delta_now`) 1e-05)) (/ (`KismetMathLibrary.VSize` _returnvalue) (+ (`self.delta_last`) 1e-05))) 2.0) 100.0)))
    (:`then_3`
      (return (`local.velo_vector`) (`local.velo_value`)))))