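; Haptic hub actor that turns musical pitches into pulses on a haptic vest and previews the motors as meshes.
; PlayPitch wraps a pitch into twelve note classes and sets the mapped motor in VestState to full intensity.
; Tick decays all intensities, rescales the meshes to match, and sends the state through PlayDot if haptic feedback is on.
; The construction script spaces one mesh per note mapping along a spline.
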(event `self.ReceiveTick`
  (params (DeltaSeconds :type "Float (single-precision)"))
  (bind _vest_state (`self.vest_state`))
  ;[1 1 1] sinusoidy krążą po plecach
  (`|ExecutionSequence`
    (:`then_0`
      (for (_array_element _array_index) _vest_state
        (`KismetArrayLibrary.Array_Set` _vest_state _array_index (`KismetMathLibrary.FFloor` (`KismetMathLibrary.FClamp` (- (`KismetMathLibrary.Conv_IntToDouble` _array_element) (* DeltaSeconds (`self.fallback_power`))) 0.0 100.0)))))
    (:`then_1`
      (`self.update_repr` _vest_state))
    (:`then_2`
      (`self.dot_play_wrapper` _vest_state))))

(fn `dot_play_wrapper`
  (params (motorValues :type "Array of Integer"))
  (if (`self.haptic_feedback_on`)
    (`BhapticsSDK2.PlayDot` 0 motorValues 0.1)))

(fn `play_pitch`
  (params (pitch :type "Float (double-precision)"))
  (`KismetArrayLibrary.Array_Set` (`self.vest_state`) (`|GetArrayItem` (`self.sound_2_motor_idx`) (mod (+ (`KismetMathLibrary.Round` pitch) (* 12 100)) 12)) 100))

(fn `update_repr`
  (params (haptic_state :type "Array of Integer"))
  (locals (log :type String))
  (for (_array_element _array_index) (`self.sound_2_motor_idx`)
    (`SceneComponent.SetWorldScale3D` (`|GetArrayItem` (`self.motor_representation`) _array_index) (`KismetMathLibrary.Conv_DoubleToVector` (`KismetMathLibrary.FMax` (/ (`KismetMathLibrary.Conv_IntToDouble` (`|GetArrayItem` haptic_state _array_element)) 100.0) (`self.minimal_size`))))))

(fn `UserConstructionScript`
  (bind _minimal_size (`self.minimal_size`))
  (bind _spline (`self.Spline`))
  (for (_ _array_index) (`self.sound_2_motor_idx`)
    (bind _returnvalue (* (`self.node_spacing`) _array_index))
    (bind _returnvalue_2 (`AddComponent|NODE_AddStaticMeshComponent-0` :`RelativeTransform` (`KismetMathLibrary.MakeTransform` (+ (`KismetMathLibrary.SelectVector` (0.0 0.0 0.0) (`SplineComponent.GetLocationAtDistanceAlongSpline` _spline _returnvalue "Local") (> _returnvalue (`SplineComponent.GetSplineLength` _spline))) (`KismetMathLibrary.TransformLocation` (`SceneComponent.GetRelativeTransform` _spline))) (struct) (`KismetMathLibrary.MakeVector` _minimal_size _minimal_size _minimal_size))))
    (`KismetArrayLibrary.Array_Set` (`self.motor_representation`) _array_index _returnvalue_2 true)))