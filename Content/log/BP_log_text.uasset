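; BP_log_text is an in-world log display that shows recent messages on a TextRender component.
; AddLog prefixes each message with a marker, appends it to the Logs array and drops the oldest entry once the history passes ten.
; It then concatenates the stored entries into one string and sets it as the rendered text, with no per-frame update.
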(event `/mea_vr_audio/log/BPI_logs.add_log`
  (params (message :type String))
  (`|ExecutionSequence`
    (:`then_0`
      ;[0 0 0] manage_history
      (bind _returnvalue (`KismetArrayLibrary.Array_Add` (`self.logs`) (`KismetStringLibrary.Concat_StrStr` "+++ " message " \n")))
      (if (>= _returnvalue 10)
        (`KismetArrayLibrary.Array_Remove` (`self.logs`))))
    (:`then_1`
      ;[0 0 0] cache_as_single_value
      (set `self.result` "")
      (for _array_element (`self.logs`)
        (set `self.result` (`KismetStringLibrary.Concat_StrStr` (`self.result`) _array_element)))
      ;[0 0 0] display
      (`TextRenderComponent.K2_SetText` (`self.TextRender`) (`KismetTextLibrary.Conv_StringToText` (`self.result`))))))

(fn `UserConstructionScript`)